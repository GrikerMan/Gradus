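; Base quest actor that tracks the player's objective progress for one stage of a quest.
; On BeginPlay it loads its QuestID row from DT_Quest_Data, zeroes a progress map for the current stage's objectives and binds to the player character's OnObjectiveIDCalled dispatcher.
; Each matching objective ID heard increments that entry up to its required quantity.
; Stage advancement and quest completion are not handled here.
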(event `self.ReceiveBeginPlay`
  (`self.GetQuestDetails`)
  (add `/Game/ThirdPerson/Blueprints/BP_Player.OnObjectiveIDCalled` (`/Game/QuestSystem/Interaction/Common_Function_Library.GetMyPlayerCharacter`) (`|CreateDelegate` :!event `On Objective IDHeard`)))

(fn `GetObjectionDataByID`
  (params (ObjectionID :type String))
  (returns (`Array Element` :type "/Game/QuestSystem/F_Objective_Details Structure"))
  (for _array_element (`.Objections_21_23FD33EE4388698E8E589CA646254DD5` (break `/Game/QuestSystem/F_Stage_Details` (`self.CurrentStageDetails`)))
    (if (`KismetStringLibrary.EqualEqual_StrStr` (`.ObjectiveID_9_305C960245E1783C10CB2A8DFB89216A` (break `/Game/QuestSystem/F_Objective_Details` _array_element)) ObjectionID)
      (return _array_element))))

(fn `GetQuestDetails`
  (bind _returnvalue (`|GetDataTableRow` "/Game/QuestSystem/DT_Quest_Data.DT_Quest_Data" (`self.QuestID`))
    (:`then`
      (bind _output_get (set `self.QuestDetails` _returnvalue))
      (bind _output_get_2 (set `self.CurrentStageDetails` (`|GetArrayItem` (`.Stages_17_B34DF5FC485ECD2E86610498128D8062` (break `/Game/QuestSystem/F_Quest_Details` _output_get)) (`self.Current Stage`))))
      (`BlueprintMapLibrary.Map_Clear` (`self.CurrentObjectiveProgress`))
      (for _array_element (`.Objections_21_23FD33EE4388698E8E589CA646254DD5` (break `/Game/QuestSystem/F_Stage_Details` _output_get_2))
        (`BlueprintMapLibrary.Map_Add` (`self.CurrentObjectiveProgress`) (`.ObjectiveID_9_305C960245E1783C10CB2A8DFB89216A` (break `/Game/QuestSystem/F_Objective_Details` _array_element)))))))

(fn `On Objective IDHeard`
  (params (`Objective ID` :type String))
  (bind (_value _returnvalue) (`BlueprintMapLibrary.Map_Find` (`self.CurrentObjectiveProgress`) `Objective ID`))
  (if _returnvalue
    (if (< _value (`.Quantity_12_2C1A6D2E4E4B4107B9978292A5A16BC2` (break `/Game/QuestSystem/F_Objective_Details` (`self.GetObjectionDataByID` `Objective ID`))))
      (`BlueprintMapLibrary.Map_Add` (`self.CurrentObjectiveProgress`) (`local.Objective ID`) (+ _value 1))
      (return))
    (else
      (return))))

(fn `UserConstructionScript`)