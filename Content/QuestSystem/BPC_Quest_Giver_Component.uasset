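; Actor component for quest givers that offers its assigned quest when the player interacts with it.
; InteractWith asks the player's quest log component whether the quest is already active, printing a notice if so.
; Otherwise, DisplayQuest looks up the quest's data table row and shows a W_Quest_Giver widget with its details and ID.
; Both paths return the owner's display name as a Name.
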(event `InteractWith`
  (params (PlayerCharacter :type "/Game/ThirdPerson/Blueprints/BP_Player Object Reference")))

(fn `DisplayQuest`
  (bind (_questdata_datatable _questdata_rowname) (break `DataTableRowHandle` (`self.QuestData`)))
  (bind _returnvalue (`|GetDataTableRow` _questdata_datatable _questdata_rowname)
    (:`then`
      (bind _returnvalue_2 (`|CreateWidget` "/Game/QuestSystem/UI/W_Quest_Giver.W_Quest_Giver_C" null _returnvalue _questdata_rowname))
      (`UserWidget.AddToViewport` _returnvalue_2 0))))

(fn `Interact With`
  (returns (ObjectiveID :type Name))
  (bind (_questdata_datatable _questdata_rowname) (break `DataTableRowHandle` (`self.QuestData`)))
  (bind _returnvalue (`KismetSystemLibrary.GetDisplayName` (`self.GetOwner`)))
  (if (not (`/Game/QuestSystem/BPC_Quest_Log_Component.QueryActiveQuest` (`/Game/ThirdPerson/Blueprints/BP_Player.BPC_Quest_Log_Component` (`/Game/QuestSystem/Interaction/Common_Function_Library.GetMyPlayerCharacter`)) _questdata_rowname))
    (`self.DisplayQuest`)
    (return (`KismetStringLibrary.Conv_StringToName` _returnvalue))
    (else
      (`KismetSystemLibrary.PrintString` "Already on Quest")
      (return (`KismetStringLibrary.Conv_StringToName` _returnvalue)))))