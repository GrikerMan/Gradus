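; BPC_DamageSystem is a component that manages an actor's health, death, healing and stun meter.
; TakeDamage reports a damage event for AI sensing and restarts a one-second recently-damaged flag, even if CanBeDamaged then blocks the hit for death or invincibility.
; Damage clamps health and signals death, or, when interruptible or forced, drains stun and dispatches the hit's response, substituting another response when stun depletes.
; ResetStunMeter restores stun to maximum.
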(event `WasDamagedTimer`
  (set `self.WasDamagedInLastSecond` true)
  (bind _returnvalue (`KismetSystemLibrary.K2_SetTimerDelegate` (delegate `ResetBool`) 1.0))
  (set `self.TimerForDamageReceived` _returnvalue))

(event `ResetBool`
  (set `self.WasDamagedInLastSecond` false))

(fn `Heal`
  (params (HealAmount :type "Float (double-precision)"))
  (returns (NewHealth :type "Float (double-precision)"))
  (if (not (`self.isDead`))
    (bind _output_get (set `self.CurrentHealth` (`KismetMathLibrary.FClamp` (+ HealAmount (`self.CurrentHealth`)) 0.0 (`self.MaxHealth`))))
    (return _output_get)))

(fn `ResetStunMeter`
  (set `self.CurrentStun` (`self.MaxStun`)))

(fn `TakeDamage`
  (params (DamageInfo :type "/Game/DamageSystem/S_DamageInfo Structure"))
  (returns (wasDamaged :type Boolean))
  (bind (_damage _stunmeteramount _knockbackamount _damagetype _damageresponse _shoulddamageinvincible _shouldforceinterrupt _actorwhodamaged) (break `/Game/DamageSystem/S_DamageInfo` DamageInfo))
  (`AISense_Damage.ReportDamageEvent` (`self.GetOwner`) _actorwhodamaged 0.0 (`Actor.K2_GetActorLocation` (`self.GetOwner`)))
  (`KismetSystemLibrary.K2_ClearAndInvalidateTimerHandle` (`self.TimerForDamageReceived`))
  (`self.WasDamagedTimer`)
  (`self.CanBeDamaged` _shoulddamageinvincible
    (:`DoDamage`
      (bind _output_get (set `self.CurrentHealth` (`KismetMathLibrary.FClamp` (- (`self.CurrentHealth`) _damage) 0.0 (`self.MaxHealth`))))
      (if (<= _output_get 0.0)
        (set `self.isDead` true)
        (`self.OnDeath`)
        (return true)
        (elif (or (`self.isInterruptible`) _shouldforceinterrupt)
          (bind _output_get_2 (set `self.CurrentStun` (- (`self.CurrentStun`) _stunmeteramount)))
          (if (<= _output_get_2 0.0)
            (`self.OnDamageRespone` "NewEnumerator2")
            (else
              (`self.OnDamageRespone` _damageresponse)))
          (return true))))
    (:`NoDamage`
      (return false))))