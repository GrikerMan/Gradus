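; Ranged enemy Blueprint that damages the AI controller's attack target from a distance.
; Attack line-traces on Visibility to the target with debug drawing, sends damage and stun only if nothing is hit, then signals attack end after a short delay.
; It also supplies walk speeds per movement state and ideal attack and defend radii.
; An unconnected workaround for broken spawning would relocate a BP_Glühwürmchen and set it attacking the player.
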(event `/Game/Enemy/AI/BPI_EnemyAI.Attack`
  (bind _asaic_enemy_base (cast `/Game/Enemy/AI/AIC_EnemyBase` (`AIBlueprintHelperLibrary.GetAIController` self)))
  (bind _attacktarget (`/Game/Enemy/AI/AIC_EnemyBase.AttackTarget` _asaic_enemy_base)
    (:`then`
      (bind (_outhit _returnvalue) (`KismetSystemLibrary.LineTraceSingle` :`Start` (`self.K2_GetActorLocation` self) :`End` (`self.K2_GetActorLocation` _attacktarget) :`TraceChannel` "TraceTypeQuery1" :`DrawDebugType` "ForDuration" :`DrawTime` 2.0))
      (if (not _returnvalue)
        (message `/Game/DamageSystem/BPI_Damagable.TakeDamage` _attacktarget (make `/Game/DamageSystem/S_DamageInfo` 10.0 50.0 0.0 "NewEnumerator2")))
      (`KismetSystemLibrary.Delay` 0.2)
      (`self.OnAttackEnd`))
    (:`else`)))

(fn `GetIdealRanges`
  (returns (AttackRadius :type "Float (double-precision)") (DefendRadius :type "Float (double-precision)"))
  (return 600.0 600.0))

(fn `SetMovementSpeed`
  (params (Speed :type "/Game/Enemy/AI/Enums/E_MovementSpeed Enum" :default "NewEnumerator0"))
  (returns (SpeedValue :type "Float (double-precision)"))
  (bind _output_get (set `CharacterMovementComponent.MaxWalkSpeed` (select `/Game/Enemy/AI/Enums/E_MovementSpeed` Speed :`NewEnumerator1` 200.0 :`NewEnumerator4` 300.0 :`NewEnumerator2` 500.0 :!type "Float (single-precision)") (`self.CharacterMovement`)))
  (return _output_get))

(fn `UserConstructionScript`
  (`parent.UserConstructionScript`))