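; BP_Enemy is a melee enemy character driven by an AIC_EnemyBase behaviour tree, with world health and stun widgets.
; BPCDamageSystem handles health, stun, damage and death, exposed through getters alongside patrol route, ideal ranges and movement speed setters.
; A stun response pauses AI logic briefly, attacks play a sword montage, and hits add knockback.
; Death stops the AI, hides widgets, clears player lock-on, ragdolls, then destroys the actor.
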(event `self.ReceiveBeginPlay`
  ;[0.05098 0.05098 0.05098] BeginPlay
  (bind _asaic_enemy_base (cast `/Game/Enemy/AI/AIC_EnemyBase` (`AIBlueprintHelperLibrary.GetAIController` self)))
  (set `self.AICEnemyBase` _asaic_enemy_base)
  (`|ExecutionSequence`
    (:`then_0`
      (bind _returnvalue (`|CreateWidget` "/Game/DamageSystem/WB_HealthBar.WB_HealthBar_C" null self))
      (`WidgetComponent.SetWidget` (`self.HealthBar`) _returnvalue))
    (:`then_1`
      (bind _returnvalue_2 (`|CreateWidget` "/Game/DamageSystem/WB_StunMeter.WB_StunMeter_C" null self))
      (`WidgetComponent.SetWidget` (`self.StunMeter`) _returnvalue_2))))

(event `DamageResponse`
  (params (DamageResponse :type "/Game/DamageSystem/E_DamageResponse Enum" :default "NewEnumerator0"))
  (bind _braincomponent (`AIController.BrainComponent` (`AIBlueprintHelperLibrary.GetAIController` self)))
  (switch `/Game/DamageSystem/E_DamageResponse` DamageResponse
    (:`NewEnumerator2`
      (`/Engine/EditorBlueprintResources/StandardMacros.DoOnce` false :!label _label
        (:`Completed`
          (`BrainComponent.StopLogic` _braincomponent "Stun")
          (`KismetSystemLibrary.Delay` 2.0)
          (`/Game/DamageSystem/BPC_DamageSystem.ResetStunMeter` (`self.BPC_DamageSystem`))
          (`BrainComponent.StartLogic` _braincomponent)
          (goto _label :!via `Reset`))))))

(event `/Game/Enemy/AI/BPI_EnemyAI.Attack`
  (`|PlayMontage` (`self.Mesh`) "/Game/Animations/MixamoCharacter/Stable_Sword_Outward_Slash__1__Anim_mixamo_com_Montage1.Stable_Sword_Outward_Slash__1__Anim_mixamo_com_Montage1"
    (:`OnCompleted`
      _)
    (:`OnInterrupted`
      _))
  (`self.OnAttackEnd`))

(event `/Game/DamageSystem/BPI_Damagable.Death`
  (`self.DeathFunctionality`))

(event `DeathFunctionality`
  (bind _aicenemybase (`self.AICEnemyBase`))
  (bind _mesh (`self.Mesh`))
  ;[1 1 1] stop behaviour tree
  (`/Game/Enemy/AI/AIC_EnemyBase.SetStateAsDead` _aicenemybase null)
  (`KismetSystemLibrary.Delay` 0.1)
  (`BrainComponent.StopLogic` (`AIController.BrainComponent` _aicenemybase) "Alkoholvergiftung")
  ;[1 1 1] hide everything visible
  (`SceneComponent.SetVisibility` (`self.StunMeter`) false false)
  (`SceneComponent.SetVisibility` (`self.HealthBar`) false false)
  (`SceneComponent.SetVisibility` (`self.LockImage`) false false)
  ;[1 1 1] remove camera lock
  (bind _asbp_player (cast `/Game/ThirdPerson/Blueprints/BP_Player` (`GameplayStatics.GetPlayerCharacter` 0)))
  (set `/Game/ThirdPerson/Blueprints/BP_Player.LockedOnTarget` null _asbp_player)
  ;[1 1 1] death animation
  (`PrimitiveComponent.SetSimulatePhysics` _mesh true)
  (`PrimitiveComponent.SetCollisionEnabled` _mesh "QueryAndPhysics")
  ;[1 1 1] wait and destroy actor
  (`KismetSystemLibrary.Delay` 2.0)
  (`self.K2_DestroyActor`))

(event `StartTimer`
  (params (Time :type "Float (double-precision)"))
  ;[1 0.5507 0.3378] trash timer, can be used for anything
  (`/Engine/EditorBlueprintResources/StandardMacros.DoOnce` false
    (:`Completed`
      (`KismetSystemLibrary.K2_SetTimerDelegate` (delegate `SetTimeIsOverToTrue`) Time))))

(event `SetTimeIsOverToTrue`
  ;[1 0.5507 0.3378] trash timer, can be used for anything
  (set `self.TimeIsOver` true))

(fn `GetCurrentHealth`
  (returns (CurrentHealth :type "Float (double-precision)"))
  (return (`/Game/DamageSystem/BPC_DamageSystem.CurrentHealth` (`self.BPC_DamageSystem`))))

(fn `GetCurrentStunMeter`
  (returns (CurrentStunMeter :type "Float (double-precision)"))
  (return (`/Game/DamageSystem/BPC_DamageSystem.CurrentStun` (`self.BPC_DamageSystem`))))

(fn `GetIdealRanges`
  (returns (AttackRadius :type "Float (double-precision)") (DefendRadius :type "Float (double-precision)"))
  (return 150.0 350.0))

(fn `GetMaxHealth`
  (returns (MaxHealth :type "Float (double-precision)"))
  (return (`/Game/DamageSystem/BPC_DamageSystem.MaxHealth` (`self.BPC_DamageSystem`))))

(fn `GetMaxStunMeter`
  (returns (MaxStunMeter :type "Float (double-precision)"))
  (return (`/Game/DamageSystem/BPC_DamageSystem.MaxStun` (`self.BPC_DamageSystem`))))

(fn `GetPatrolRoute`
  (returns (PatrolRoute :type "/Game/Enemy/AI/BP_PatrolRoute Object Reference"))
  (return (`self.PatrolRoute`)))

(fn `GetWasDamagedInLastSecondBool`
  (returns (WasDamagedInLastSecond :type Boolean))
  (return (`/Game/DamageSystem/BPC_DamageSystem.WasDamagedInLastSecond` (`self.BPC_DamageSystem`))))

(fn `Heal`
  (params (HealAmount :type "Float (double-precision)"))
  (returns (NewHealth :type "Float (double-precision)"))
  (bind _newhealth (`/Game/DamageSystem/BPC_DamageSystem.Heal` (`self.BPC_DamageSystem`) HealAmount))
  (return _newhealth))

(fn `IsDead`
  (returns (Dead :type Boolean))
  (return (`/Game/DamageSystem/BPC_DamageSystem.isDead` (`self.BPC_DamageSystem`))))

(fn `SetMovementSpeed`
  (params (Speed :type "/Game/Enemy/AI/Enums/E_MovementSpeed Enum" :default "NewEnumerator0"))
  (returns (SpeedValue :type "Float (double-precision)"))
  (bind _output_get (set `CharacterMovementComponent.MaxWalkSpeed` (select `/Game/Enemy/AI/Enums/E_MovementSpeed` Speed :`NewEnumerator1` 100.0 :`NewEnumerator4` 300.0 :`NewEnumerator2` 500.0 :!type "Float (single-precision)") (`self.CharacterMovement`)))
  (return _output_get))

(fn `TakeDamage`
  (params (DamageInfo :type "/Game/DamageSystem/S_DamageInfo Structure"))
  (returns (wasDamaged :type Boolean))
  (bind (_damage _stunmeteramount _knockbackamount _damagetype _damageresponse _shoulddamageinvincible _shouldforceinterrupt _actorwhodamaged) (break `/Game/DamageSystem/S_DamageInfo` DamageInfo))
  (bind _wasdamaged (`/Game/DamageSystem/BPC_DamageSystem.TakeDamage` (`self.BPC_DamageSystem`) DamageInfo))
  (`self.LaunchCharacter` (* (`self.GetActorForwardVector` _actorwhodamaged) _knockbackamount))
  (return _wasdamaged))

(fn `UserConstructionScript`
  (bind _bpc_damagesystem (`self.BPC_DamageSystem`))
  (add `/Game/DamageSystem/BPC_DamageSystem.OnDamageRespone` _bpc_damagesystem (`|CreateDelegate` :!event `DamageResponse`))
  (add `/Game/DamageSystem/BPC_DamageSystem.OnDeath` _bpc_damagesystem (`|CreateDelegate` :!event `Death`)))