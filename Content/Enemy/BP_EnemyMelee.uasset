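; Melee enemy Blueprint that performs a sword slash when its Attack event fires.
; Attack plays the slash montage, and each notify begin sphere-traces a short distance forward for Pawn objects, with debug drawing enabled.
; A hit actor receives a fixed-damage struct with no stun through the TakeDamage interface message.
; Montage completion or interruption both call OnAttackEnd to signal that the attack is over.
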(event `/Game/Enemy/AI/BPI_EnemyAI.Attack`
  (bind _returnvalue (`self.K2_GetActorLocation`))
  (bind _notifyname (`|PlayMontage` (`self.Mesh`) "/Game/Animations/MixamoCharacter/Stable_Sword_Outward_Slash__1__Anim_mixamo_com_Montage1.Stable_Sword_Outward_Slash__1__Anim_mixamo_com_Montage1")
    (:`OnCompleted`
      (`self.OnAttackEnd` :!label _label))
    (:`OnInterrupted`
      (goto _label))
    (:`OnNotifyBegin`
      (switch `name` _notifyname
        (:`Slash`
          (bind (_outhit _returnvalue_2) (`KismetSystemLibrary.SphereTraceSingleForObjects` :`Start` _returnvalue :`End` (+ _returnvalue (* (`self.GetActorForwardVector`) 200.0)) :`Radius` 20.0 :`ObjectTypes` (`|MakeArray` "ObjectTypeQuery3" :!type "EObjectTypeQuery Enum") :`DrawDebugType` "ForDuration" :`DrawTime` 2.0))
          (if _returnvalue_2
            (message `/Game/DamageSystem/BPI_Damagable.TakeDamage` (`.HitActor` (`GameplayStatics.BreakHitResult` _outhit)) (make `/Game/DamageSystem/S_DamageInfo` 30.0 0.0 0.0 "NewEnumerator1" "NewEnumerator2"))))))))

(fn `UserConstructionScript`
  (`parent.UserConstructionScript`))