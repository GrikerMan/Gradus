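; Chain projectile for the player's metal ability that hooks actors and drags them toward the player.
; It launches toward the EndLocation from BPC_MetalAbility, then Tick pulls it back toward the player once it arrives.
; During retraction, the first capsule end-overlap attaches and damages that actor, which detaches within EnemyDistance of the player.
; On reaching the updated StartLocation, it clears the component's HasSpawned flag and destroys itself.
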(event `self.ReceiveBeginPlay`
  (`|ExecutionSequence`
    (:`then_0`
      (`self.GetReferences`))
    (:`then_1`
      (add `PrimitiveComponent.OnComponentEndOverlap` (`self.Capsule`) (delegate `OnChainEndOveralp`))
      (`self.ExtractChain`))))

(event `OnChainEndOveralp`
  (params (OverlappedComponent :type "PrimitiveComponent Object Reference") (OtherActor :type "Actor Object Reference") (OtherComp :type "PrimitiveComponent Object Reference") (OtherBodyIndex :type Integer))
  ;[1 1 1] On Overlap
  (set `self.OverlapActor` OtherActor)
  (`self.HandleOnOverlap` OtherActor))

(event `self.ReceiveTick`
  (params (DeltaSeconds :type "Float (single-precision)"))
  (`|ExecutionSequence`
    (:`then_0`
      (`self.UpdateStartLocation`)
      ;[1 1 1] Retract Chain
      (`self.StopExtraction`))
    (:`then_1`
      (if (`self.IsOut`)
        (`|ExecutionSequence`
          (:`then_0`
            (`self.StopRetraction`))
          (:`then_1`
            (`self.Retract Chain`)))))
    (:`then_2`
      (`self.DetachEnemy`))))

(fn `DetachEnemy`
  (if (and (`self.IsEnemyHooked`) (`self.IsOut`))
    (if (<= (`KismetMathLibrary.VSize` (`self.GetDistanceBetweenPlayerAndChain`)) (`self.EnemyDistance`))
      (`self.K2_DetachFromActor` (`self.OverlapActor`) "KeepWorld" "KeepWorld" "KeepWorld")
      (return))))

(fn `ExtractChain`
  (`self.K2_SetActorRotation` (`self.RotationToTarget`))
  (`ActorComponent.Activate` (`self.ProjectileMovement`) false)
  (`ProjectileMovementComponent.SetVelocityInLocalSpace` (`self.ProjectileMovement`) (`KismetMathLibrary.MakeVector` (`self.ExtractSpeed`)))
  (return))

(fn `GetDistanceBetweenPlayerAndChain`
  (returns (DistancePlayerChain :type "Vector Structure"))
  (return (- (`SceneComponent.K2_GetComponentLocation` (`Actor.RootComponent` (`self.BPPlayerReference`))) (`self.K2_GetActorLocation` self))))

(fn `GetReferences`
  (bind _asbp_player (cast `/Game/ThirdPerson/Blueprints/BP_Player` (`GameplayStatics.GetPlayerCharacter` 0)))
  (set `self.BPPlayerReference` _asbp_player)
  (bind _returnvalue (`self.GetComponentByClass` _asbp_player "/Game/Gradus/Core/MetalAbility/BPC_MetalAbility.BPC_MetalAbility_C"))
  (set `self.BPCMetalAbilityReference` _returnvalue)
  (set `self.EndLocation` (`/Game/Gradus/Core/MetalAbility/BPC_MetalAbility.EndLocation` _returnvalue))
  (set `self.RotationToTarget` (`/Game/Gradus/Core/MetalAbility/BPC_MetalAbility.RotationToTarget` _returnvalue))
  (return))

(fn `HandleOnOverlap`
  (params (OtherActor :type "Actor Object Reference"))
  (if (`self.IsOut`)
    (`/Engine/EditorBlueprintResources/StandardMacros.DoOnce` false
      (:`Completed`
        (`self.K2_AttachToActor` (`local.OtherActor`) self "None" "KeepWorld" "KeepWorld" "KeepWorld" true)
        (set `self.IsEnemyHooked` true)
        (message `/Game/DamageSystem/BPI_Damagable.TakeDamage` (`local.OtherActor`) (make `/Game/DamageSystem/S_DamageInfo` (`self.Damage`) 0.0 0.0 "NewEnumerator3" "NewEnumerator0" false false self))
        (return)))))

(fn `Retract Chain`
  (bind _returnvalue (`KismetMathLibrary.Normal` (`self.GetDistanceBetweenPlayerAndChain`)))
  (`/Engine/EditorBlueprintResources/StandardMacros.IsValid` self
    (:`Is Valid`
      (`self.K2_AddActorWorldOffset` (* _returnvalue (`self.RetractSpeed`)))
      (`self.K2_SetActorRotation` (`KismetMathLibrary.MakeRotFromX` (`KismetMathLibrary.NegateVector` _returnvalue)))
      (return))))

(fn `StopExtraction`
  (if (== (`self.K2_GetActorLocation` self) (`self.EndLocation`) :`ErrorTolerance` 50.0)
    (`/Engine/EditorBlueprintResources/StandardMacros.DoOnce` false
      (:`Completed`
        (`MovementComponent.StopMovementImmediately` (`self.ProjectileMovement`))
        (set `self.IsOut` true)
        (return)))))

(fn `StopRetraction`
  (if (== (`self.K2_GetActorLocation` self) (`self.StartLocation`) :`ErrorTolerance` 50.0)
    (`/Engine/EditorBlueprintResources/StandardMacros.DoOnce` false
      (:`Completed`
        (`MovementComponent.StopMovementImmediately` (`self.ProjectileMovement`))
        (set `/Game/Gradus/Core/MetalAbility/BPC_MetalAbility.HasSpawned` false (`self.BPCMetalAbilityReference`))
        (set `self.IsEnemyHooked` false)
        (set `self.IsOut` false)
        (`self.K2_DestroyActor`)
        (return)))))

(fn `UpdateStartLocation`
  (set `self.StartLocation` (`/Game/Gradus/Core/MetalAbility/BPC_MetalAbility.StartLocation` (`self.GetComponentByClass` (`self.BPPlayerReference`) "/Game/Gradus/Core/MetalAbility/BPC_MetalAbility.BPC_MetalAbility_C")))
  (return))

(fn `UserConstructionScript`)