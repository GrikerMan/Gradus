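; BP_MetalBolt is a metal-ability projectile that damages the character it hits and sticks into its body.
; The first overlap whose actor yields a skeletal mesh triggers, after a very brief delay, a one-time hit handler.
; The handler stops projectile movement, attaches the bolt to the closest bone keeping its world transform, sends a damage message, and sets a timed lifespan for cleanup.
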(event `self.ReceiveBeginPlay`
  (add `PrimitiveComponent.OnComponentBeginOverlap` (`self.MetalBoltMesh`) (delegate `CustomEvent`)))

(event `CustomEvent`
  (params (OverlappedComponent :type "PrimitiveComponent Object Reference") (OtherActor :type "Actor Object Reference") (OtherComp :type "PrimitiveComponent Object Reference") (OtherBodyIndex :type Integer) (bFromSweep :type Boolean) (SweepResult :type "HitResult Structure (by ref)"))
  (bind _asskeletal_mesh_component (cast `SkeletalMeshComponent` (`self.GetComponentByClass` OtherActor "/Script/Engine.MeshComponent")))
  (`/Engine/EditorBlueprintResources/StandardMacros.DoOnce` false
    (:`Completed`
      (`KismetSystemLibrary.Delay` 0.015)
      (`self.Handle on Overlap` OtherActor _asskeletal_mesh_component))))

(fn `Handle on Overlap`
  (params (OtherActor :type "Actor Object Reference") (SkeletalMeshComponent :type "SkeletalMeshComponent Object Reference"))
  (bind _skeletalmeshcomponent (`local.SkeletalMeshComponent`))
  (`ActorComponent.Deactivate` (`self.ProjectileMovement`))
  (`self.K2_AttachToComponent` self _skeletalmeshcomponent (`.ReturnValue` (`SkinnedMeshComponent.FindClosestBone_K2` _skeletalmeshcomponent (`self.K2_GetActorLocation` self) 0.0 false)) "KeepWorld" "KeepWorld" "KeepWorld" true)
  (message `/Game/DamageSystem/BPI_Damagable.TakeDamage` (`local.OtherActor`) (make `/Game/DamageSystem/S_DamageInfo` (`self.Damage`) 0.0 0.0 "NewEnumerator3" "NewEnumerator0" false false self))
  (`self.SetLifeSpan` 10.0)
  (return))

(fn `UserConstructionScript`)