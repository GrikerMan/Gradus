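; Player component for the metal ability, with bolt and chain modes that the switch input toggles after resetting the current state.
; In bolt mode, shooting spawns bolts on mesh sockets, launches them in random order toward the camera's line-trace target, then respawns once all are fired.
; In chain mode, shooting spawns one BP_Chain per reset, aimed by camera sphere trace, with its cable end attached to a character socket.
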(event `self.ReceiveBeginPlay`
  ;[1 1 1] Get References
  (`self.GetPlayerReferences`))

(event `EnhancedInput|/Game/ThirdPerson/Input/Actions/IA_Shoot`
  (params (ActionValue :type Boolean) (ElapsedSeconds :type "Float (double-precision)") (TriggeredSeconds :type "Float (double-precision)") (InputAction :type "InputAction Object Reference" :default "/Game/ThirdPerson/Input/Actions/IA_Shoot.IA_Shoot"))
  (:`Triggered`
    (if (`self.IsFruitPositive`)
      _
      (elif (`self.HasSpawnedAndInBoltRange`)
        ;[1 1 1] Shoot Bolt
        (`self.GetRandomBolt`)
        (`Actor.K2_DetachFromActor` (`self.MetalBoltReference`) "KeepWorld" "KeepWorld" "KeepWorld")
        (bind _returnvalue (`self.GetBoltRotation`))
        (`self.SetDirectionandFire` _returnvalue)
        (else
          ;[1 1 1] Spawn Bolts
          (for _array_element (`self.BoltSocketNames`)
            (`self.SpawnBolt` _array_element))
          (set `self.TraceDistance` (`self.BoltRange`))
          (set `self.BoltsShot` 0)
          (set `self.HasSpawned` true)))))
  (:`Started`
    (if (`self.IsFruitPositive`)
      ;[1 1 1] Spawn Chain
      (if (not (`self.HasSpawned`))
        (set `self.HasSpawned` true)
        (set `self.TraceDistance` (`self.ChainRange`))
        (`self.SpawnChain`)))))

(event `self.ReceiveTick`
  (params (DeltaSeconds :type "Float (single-precision)"))
  ;[1 1 1] Update Chain StartLocation
  (`KismetSystemLibrary.Delay` 0.1)
  (`self.UpdateChainStartLocation`))

(event `EnhancedInput|/Game/ThirdPerson/Input/Actions/IA_SwitchAbility`
  (params (ActionValue :type Boolean) (ElapsedSeconds :type "Float (double-precision)") (TriggeredSeconds :type "Float (double-precision)") (InputAction :type "InputAction Object Reference" :default "/Game/ThirdPerson/Input/Actions/IA_SwitchAbility.IA_SwitchAbility"))
  (:`Started`
    ;[1 1 1] Switch Ability
    (`self.ResetAbilities`)
    (if (`self.IsFruitPositive`)
      (set `self.IsFruitPositive` false)
      (else
        (set `self.IsFruitPositive` true)))))

(fn `AddOffsetToImpactPoint`
  (params (ImpactPoint :type "Vector Structure") (TraceEnd :type "Vector Structure"))
  (returns (ReturnValue :type "Vector Structure"))
  (return (+ (`local.ImpactPoint`) (* (`KismetMathLibrary.Normal` (- (`local.TraceEnd`) (`local.ImpactPoint`))) 15.0))))

(fn `GetBoltRotation`
  (returns (ReturnValue :type "Rotator Structure"))
  (locals (TraceEnd :type "Vector Structure"))
  (bind _output_get (set `local.TraceEnd` (`self.GetTraceEnd`)))
  (bind _outhit (`KismetSystemLibrary.LineTraceSingle` (`SceneComponent.K2_GetComponentLocation` (`self.CameraReference`)) _output_get "TraceTypeQuery2" false (`|MakeArray` (`GameplayStatics.GetPlayerCharacter` 0) :!type "Actor Object Reference")))
  (bind (_bblockinghit _binitialoverlap _time _distance _location _impactpoint) (`GameplayStatics.BreakHitResult` _outhit))
  (return (`KismetMathLibrary.FindLookAtRotation` (`Actor.K2_GetActorLocation` (`self.MetalBoltReference`)) (`KismetMathLibrary.SelectVector` _impactpoint (`local.TraceEnd`) _bblockinghit))))

(fn `GetChainSpawnTransform`
  (returns (ReturnValue :type "Transform Structure"))
  (locals (TraceEnd :type "Vector Structure"))
  (bind _returnvalue (`self.GetTraceEnd`))
  (bind _traceend (`local.TraceEnd`))
  (set `local.TraceEnd` _returnvalue)
  (bind _outhit (`KismetSystemLibrary.SphereTraceSingle` :`Start` (`SceneComponent.K2_GetComponentLocation` (`self.CameraReference`)) :`End` _returnvalue :`Radius` 10.0 :`TraceChannel` "TraceTypeQuery2" :`DrawTime` 10.0))
  (bind (_bblockinghit _binitialoverlap _time _distance _location _impactpoint) (`GameplayStatics.BreakHitResult` _outhit))
  (bind _returnvalue_2 (`KismetMathLibrary.SelectVector` (`self.AddOffsetToImpactPoint` _impactpoint _traceend) _traceend _bblockinghit))
  (set `self.EndLocation` _returnvalue_2)
  (bind _returnvalue_3 (`KismetMathLibrary.FindLookAtRotation` (`self.StartLocation`) _returnvalue_2))
  (set `self.RotationToTarget` _returnvalue_3)
  (return (`KismetMathLibrary.MakeTransform` (`self.StartLocation`) _returnvalue_3)))

(fn `GetPlayerReferences`
  (bind _asbp_player (cast `/Game/ThirdPerson/Blueprints/BP_Player` (`self.GetOwner`)))
  (set `self.CameraReference` (`/Game/ThirdPerson/Blueprints/BP_Player.FollowCamera` _asbp_player))
  (set `self.CharacterMeshReference` (`Character.Mesh` _asbp_player))
  (return))

(fn `GetRandomBolt`
  (bind _asbp_metal_bolt (cast `/Game/Gradus/Core/MetalAbility/BP_MetalBolt` (`KismetArrayLibrary.Array_Random` (`self.MetalBolts`))))
  (bind _output_get (set `self.MetalBoltReference` _asbp_metal_bolt))
  (`KismetArrayLibrary.Array_RemoveItem` (`self.MetalBolts`) _output_get)
  (return))

(fn `GetTraceEnd`
  (returns (ReturnValue :type "Vector Structure"))
  (bind _camerareference (`self.CameraReference`))
  (return (+ (`SceneComponent.K2_GetComponentLocation` _camerareference) (* (`SceneComponent.GetForwardVector` _camerareference) (`self.TraceDistance`)))))

(fn `HasSpawnedAndInBoltRange`
  (returns (ReturnValue :type Boolean))
  (return (and (`self.HasSpawned`) (<= (`self.BoltsShot`) (- (`KismetArrayLibrary.Array_Length` (`self.BoltSocketNames`)) 1)))))

(fn `ResetAbilities`
  (for _array_element (`self.MetalBolts`)
    (`Actor.K2_DestroyActor` _array_element))
  (set `self.HasSpawned` false)
  (`KismetArrayLibrary.Array_Clear` (`self.MetalBolts`))
  (return))

(fn `SetDirectionandFire`
  (params (NewRotation :type "Rotator Structure"))
  (bind _returnvalue (`Actor.GetComponentByClass` (`self.MetalBoltReference`) "/Script/Engine.ProjectileMovementComponent"))
  (`Actor.K2_SetActorRotation` (`self.MetalBoltReference`) NewRotation false)
  (`ProjectileMovementComponent.SetVelocityInLocalSpace` _returnvalue (`KismetMathLibrary.MakeVector` (`self.BoltSpeed`)))
  (`self.Activate` _returnvalue false)
  (`Actor.SetLifeSpan` (`self.MetalBoltReference`) 5.0)
  (`/Engine/EditorBlueprintResources/StandardMacros.IncrementInt` (`self.BoltsShot`)
    (:`  `
      (return))))

(fn `SpawnBolt`
  (params (InSocketName :type Name))
  (bind _returnvalue (`|SpawnActorFromClass` "/Game/Gradus/Core/MetalAbility/BP_MetalBolt.BP_MetalBolt_C" (`SceneComponent.GetSocketTransform` (`self.CharacterMeshReference`) InSocketName "RTS_World") "Undefined" "MultiplyWithRoot" null null))
  (`KismetArrayLibrary.Array_Add` (`self.MetalBolts`) _returnvalue)
  (`SceneComponent.K2_AttachToComponent` (`Actor.RootComponent` _returnvalue) (`self.CharacterMeshReference`) "None" "KeepWorld" "KeepWorld" "KeepWorld" true)
  (return))

(fn `SpawnChain`
  (bind _returnvalue (`self.GetChainSpawnTransform`))
  (bind _returnvalue_2 (`|SpawnActorFromClass` "/Game/Gradus/Core/MetalAbility/BP_Chain.BP_Chain_C" _returnvalue "Undefined" "MultiplyWithRoot" null null))
  (`CableComponent.SetAttachEndToComponent` (`/Game/Gradus/Core/MetalAbility/BP_Chain.Cable` _returnvalue_2) (`self.CharacterMeshReference`) (`self.ChainSocketName`)))

(fn `UpdateChainStartLocation`
  (set `self.StartLocation` (`SceneComponent.GetSocketLocation` (`self.CharacterMeshReference`) (`self.ChainSocketName`)))
  (return))