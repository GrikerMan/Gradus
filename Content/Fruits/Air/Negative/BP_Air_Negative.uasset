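; Gameplay ability for the negative Air fruit that creates a short-lived damaging area around its user.
; On activation it commits, plays the AirNegative montage and attaches a Niagara effect to player 0's mesh, not explicitly the avatar's.
; A looping timer box-checks nearby pawns, excluding the avatar, and sends them damage and stun-meter messages.
; A second timer ends the ability after a few seconds, but the looping timer is never explicitly cleared.
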(event `CustomEvent_2`
  (`self.K2_EndAbility`))

(event `CustomEvent_0`
  (bind _returnvalue (`self.GetAvatarActorFromActorInfo`))
  (bind _outactors (`KismetSystemLibrary.BoxOverlapActors` (`Actor.K2_GetActorLocation` _returnvalue) (100.0 100.0 100.0) (`|MakeArray` "ObjectTypeQuery3" :!type "EObjectTypeQuery Enum") null (`|MakeArray` _returnvalue)))
  (for _array_element _outactors
    (message `/Game/DamageSystem/BPI_Damagable.TakeDamage` _array_element (make `/Game/DamageSystem/S_DamageInfo` 5.0 20.0))))

(event `self.K2_ActivateAbility`
  (`KismetSystemLibrary.K2_SetTimerDelegate` (delegate `CustomEvent_2`) 5.0)
  (`KismetSystemLibrary.PrintString` "Hello")
  (`self.K2_CommitAbility`)
  (`AbilityTask_PlayMontageAndWait.CreatePlayMontageAndWaitProxy` "None" (`self.Air_Negative`)
    (:`then`
      (`NiagaraFunctionLibrary.SpawnSystemAttached` "/Game/VFX/Systems/NS_DiesmalWirklichLuftFrucht.NS_DiesmalWirklichLuftFrucht" (`Character.Mesh` (`GameplayStatics.GetPlayerCharacter` 0)) "None" (0.0 0.0 90.0) (struct) "KeepRelativeOffset")
      (`KismetSystemLibrary.K2_SetTimerDelegate` (delegate `CustomEvent_0`) 0.5 true))))

(event `self.K2_OnEndAbility`
  (params (bWasCancelled :type Boolean))
  (`KismetSystemLibrary.PrintString` "Air_Negative"))

(event `CustomEvent`
  (params (DeltaSeconds :type "Float (single-precision)")))